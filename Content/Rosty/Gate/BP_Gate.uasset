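; Exit gate that ends the game with a win once it has been unlocked.
; Its trigger box starts without collision; ButtonPressed enables it and swaps the mesh to a slightly opened gate.
; After a short delay, any overlap plays the win sound and calls WinScreen on the main menu widget.
; It then appends the game mode's time to the GameInstance leaderboard with a blank name and saves.
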(event OnComponentBeginOverlap(Box)
  (params (OverlappedComponent :type Primitive%20Component%20Object%20Reference) (OtherActor :type Actor%20Object%20Reference) (OtherComp :type Primitive%20Component%20Object%20Reference) (OtherBodyIndex :type Integer) (bFromSweep :type Boolean) (SweepResult :type Hit%20Result%20Structure%20%28by%20ref%29))
  (Utilities|FlowControl|Delay 0.2)
  (bind _foundwidgets (Widget|GetAllWidgetsOfClass "/Game/Rosty/UI/WB_MainMenu.WB_MainMenu_C" true))
  (Audio|PlaySound2D "/Game/Sounds/WIN_PP.WIN_PP" 1.0 1.0 0.0 0 0)
  (Default|WinScreen _foundwidgets)
  (bind _asbp_gamemode (Utilities|Casting|CastToBP_Gamemode (Game|GetGameMode)))
  (bind _asbp_game_instance (Utilities|Casting|CastToBP_GameInstance (Game|GetGameInstance)))
  (Utilities|Array|Add (Variables|/Game/SaveSystem/BP_Leaderboard.BP_Leaderboard_C|GetThingsToSave (Variables|/Game/SaveSystem/BP_GameInstance.BP_GameInstance_C|GetCurrentLeaderboard _asbp_game_instance)) (Utilities|Struct|MakeS_ThingsToSave "" (Math|Timespan|MakeTimespan 0 0 (Variables|/Game/Conor/BP_Gamemode.BP_Gamemode_C|GetMinutes _asbp_gamemode) (Variables|/Game/Conor/BP_Gamemode.BP_Gamemode_C|GetSeconds _asbp_gamemode))))
  (Default|SavingGametoSlot _asbp_game_instance)
  (Development|PrintString "Saved!"))

(event Custom|ButtonPressed
  (Collision|SetCollisionEnabled (Variables|Default|GetBox) "QueryAndPhysics")
  (Components|StaticMesh|SetStaticMesh (Variables|Default|GetCube) "/Game/Assets/Adam/Garden/gate_sligthlyopened.gate_sligthlyopened"))

(event EventBeginPlay
  (Collision|SetCollisionEnabled (Variables|Default|GetBox) "NoCollision"))

(fn ConstructionScript)