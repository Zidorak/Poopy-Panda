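; Game mode that scatters milk bottle pickups over the level at BeginPlay and provides a minutes-and-seconds timer.
; SpawnItem picks random BP_SpawnPoint actors, spawns a BP_MilkBottle at each, then destroys the used point so none repeats.
; BeginPlay then calls FloatObject on only the first bottle found.
; StartTimer, not called here, runs a looping one-second update; Seconds is cleared only by RestartTimer, not on minute rollover.
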(event Custom|StartTimer
  (Utilities|Time|SetTimerbyEvent (delegate Custom|UpdateTimer) 1.0 true))

(event Custom|UpdateTimer
  ;[1 1 1] Seconds
  (if (== (Variables|Default|GetSeconds) 60)
    ;[1 1 1] Minutes
    (if (== (Variables|Default|GetMinutes) 60)
      (CallFunction|RestartTimer)
      (else
        (Variables|Default|SetMinutes (+ (Variables|Default|GetMinutes) 1))))
    (else
      (Variables|Default|SetSeconds (+ (Variables|Default|GetSeconds) 1)))))

(event Custom|RestartTimer
  ;[1 1 1] Restart
  (Variables|Default|SetSeconds 0)
  (Variables|Default|SetMinutes 0))

(event EventBeginPlay
  (CallFunction|SpawnItem)
  (bind _returnvalue (Actor|GetActorOfClass "/Game/Rosty/PickUps/BP_MilkBottle.BP_MilkBottle_C"))
  (Default|FloatObject _returnvalue))

(fn ConstructionScript)

(fn SpawnItem
  (bind _outactors (Actor|GetAllActorsOfClass "/Game/Rosty/PickUps/BP_SpawnPoint.BP_SpawnPoint_C"))
  (LocalVariables|SetLocalSpawnPoints _outactors)
  (for _index (range 0 3)
    (LocalVariables|SetLocal%20item (.OutItem (Utilities|Array|Random (LocalVariables|GetLocalSpawnPoints))))
    (Game|SpawnActorfromClass "/Game/Rosty/PickUps/BP_MilkBottle.BP_MilkBottle_C" (Math|Transform|MakeTransform (Transformation|GetActorLocation (LocalVariables|GetLocal%20item))) "Undefined" "MultiplyWithRoot" 0 0)
    (Utilities|Array|RemoveItem (LocalVariables|GetLocalSpawnPoints) (LocalVariables|GetLocal%20item))
    (Actor|DestroyActor (LocalVariables|GetLocal%20item))))