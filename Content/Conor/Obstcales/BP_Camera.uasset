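; BP_Camera is a security camera obstacle that alerts the adult AI and can be temporarily blinded by projectiles.
; Tick runs a delayed sphere trace from spawn point to arrow; a hit reddens the perception cone and calls SetLastKnownLocation on BP_AdultAI.
; The alarm clears and the cone turns green after a cooldown.
; A tagged projectile entering the box triggers CoveredInPoop, pausing detection and box collision for a few seconds.
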(event OnComponentBeginOverlap(Box)
  (params (OverlappedComponent :type Primitive%20Component%20Object%20Reference) (OtherActor :type Actor%20Object%20Reference) (OtherComp :type Primitive%20Component%20Object%20Reference) (OtherBodyIndex :type Integer) (bFromSweep :type Boolean) (SweepResult :type Hit%20Result%20Structure%20%28by%20ref%29))
  (if (Actor|ActorHasTag OtherActor "Projectile")
    ;[1 1 1] Spawns poop, sets col to off, sets pawn sensing to not work.
    (Class|Camera|CoveredinPoop)
    (Collision|SetCollisionEnabled (Variables|Default|GetBox) "NoCollision")
    (Variables|Default|SetIsBlinded true)
    ;[1 1 1] Reactivates all senses
    (Utilities|FlowControl|Delay 5.0)
    (Collision|SetCollisionEnabled (Variables|Default|GetBox) "QueryOnly")
    (Variables|Default|SetIsBlinded false)))

(event EventTick
  (params (DeltaSeconds :type Float%20%28single-precision%29))
  (if (not (or (Variables|Default|GetIsBlinded) (Variables|Default|GetCameraAlarmActive)))
    (Utilities|FlowControl|Delay 0.5)
    (bind (_outhit _returnvalue) (Collision|SphereTraceByChannel (Transformation|GetWorldLocation (Variables|Default|GetSpawnPoint)) (Transformation|GetWorldLocation (Variables|Default|GetArrow)) 1.5e+02 "TraceTypeQuery3" false 0 "None"))
    (if _returnvalue
      ;[1 1 1] Activates the camera alarm mechanic
      (Rendering|Material|SetMaterial (Variables|Default|GetPerceptionCone) 0 "/Game/Conor/Obstcales/PerceptionCone_Red.PerceptionCone_Red")
      (Variables|Default|SetCameraAlarmActive true)
      (bind _returnvalue_2 (Actor|GetActorOfClass "/Game/Conor/AI/BP_AdultAI.BP_AdultAI_C"))
      (Default|SetLastKnownLocation _returnvalue_2)
      ;[1 1 1] After cooldown resets the mechanic
      (Utilities|FlowControl|Delay 5.0)
      (Default|ClearCameraAlarm _returnvalue_2)
      (Variables|Default|SetCameraAlarmActive false)
      (Rendering|Material|SetMaterial (Variables|Default|GetPerceptionCone) 0 "/Game/Conor/Obstcales/PerceptionCone_Green.PerceptionCone_Green"))))

(fn ConstructionScript)