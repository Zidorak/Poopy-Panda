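; BP_Poop is a poop obstacle that stuns adult AI enemies and serves as an ammo pickup for the player.
; Its box collision overlap sorts actors by Enemy or Player tag.
; Enemies trigger CollisionHit and SetStunned on BP_AdultAI.
; Players trigger PlayerPickupAmmo and add one PooAmmo to player 0's character, fetched by index rather than from the overlapping actor.
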(event OnComponentBeginOverlap(BoxCollision)
  (params (OverlappedComponent :type Primitive%20Component%20Object%20Reference) (OtherActor :type Actor%20Object%20Reference) (OtherComp :type Primitive%20Component%20Object%20Reference) (OtherBodyIndex :type Integer) (bFromSweep :type Boolean) (SweepResult :type Hit%20Result%20Structure%20%28by%20ref%29))
  (if (Actor|ActorHasTag OtherActor "Enemy")
    (bind _asbp_adult_ai (Utilities|Casting|CastToBP_AdultAI OtherActor))
    (Class|ObstacleforAI|CollisionHit)
    (Default|SetStunned _asbp_adult_ai)
    (elif (Actor|ActorHasTag OtherActor "Player")
      (bind _asbp_player_character_true (Utilities|Casting|CastToBP_PlayerCharacterTRUE (Game|GetPlayerCharacter 0)))
      (Class|ObstacleforAI|PlayerPickupAmmo)
      (Variables|/Script/PoopyPanda.PlayerCharacterTRUE|SetPooAmmo _asbp_player_character_true (+ (Variables|/Script/PoopyPanda.PlayerCharacterTRUE|GetPooAmmo _asbp_player_character_true) 1)))))

(fn ConstructionScript)