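; Adult AI enemy character that hunts the player and shows the main menu widget's lose screen when its capsule overlaps them.
; It feeds its controller's Blackboard with target, office-role and timed stun state.
; HandleSight sets the player as target while seen and stores the last known location when sight is lost.
; Camera alerts record the player's position and temporarily change walk speed before the alarm clears.
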(event OnComponentBeginOverlap(CapsuleComponent)
  (params (OverlappedComponent :type Primitive%20Component%20Object%20Reference) (OtherActor :type Actor%20Object%20Reference) (OtherComp :type Primitive%20Component%20Object%20Reference) (OtherBodyIndex :type Integer) (bFromSweep :type Boolean) (SweepResult :type Hit%20Result%20Structure%20%28by%20ref%29))
  (if (Actor|ActorHasTag OtherActor "Player")
    (bind _foundwidgets (Widget|GetAllWidgetsOfClass "/Game/Rosty/UI/WB_MainMenu.WB_MainMenu_C" true))
    (Default|LoseScreen _foundwidgets)))

(event Custom|Set%20Last%20Known%20Location
  ;[1 1 1] Functions for the camera alert
  (Variables|/Script/Engine.CharacterMovementComponent|SetMaxWalkSpeed (Variables|Character|GetCharacterMovement) 4e+02)
  (AI|Components|Blackboard|SetValueasBool (Variables|/Script/AIModule.AIController|GetBlackboard (AI|GetAIController self)) (Utilities|Name|MakeLiteralName "CameraAlarm") true)
  (Variables|Default|SetOriginalLocation (Transformation|GetActorLocation))
  (AI|Components|Blackboard|SetValueasVector (Variables|/Script/AIModule.AIController|GetBlackboard (AI|GetAIController self)) (Utilities|Name|MakeLiteralName "LastKnownLocation") (Transformation|GetActorLocation (Game|GetPlayerCharacter 0)))
  (Utilities|FlowControl|Delay 5.0)
  (CallFunction|ClearCameraAlarm))

(event Custom|Set%20Max%20Walk%20Speed
  (params (Walk%20Speed :type Float%20%28double-precision%29))
  ;[1 1 1] Quickly set the max walking speed
  (Variables|/Script/Engine.CharacterMovementComponent|SetMaxWalkSpeed (Variables|Character|GetCharacterMovement) Walk%20Speed))

(event Custom|Set%20Stunned
  ;[1 1 1] Functions for the black board
  (AI|Components|Blackboard|SetValueasBool (AI|GetBlackboard (AI|GetAIController self)) (Utilities|Name|MakeLiteralName "Stunned") true)
  (Utilities|FlowControl|Delay (Variables|Default|GetStunnedTime))
  (AI|Components|Blackboard|SetValueasBool (AI|GetBlackboard (AI|GetAIController self)) (Utilities|Name|MakeLiteralName "Stunned") false))

(event Custom|Set%20AI%20Target
  (params (Actor :type Actor%20Object%20Reference))
  ;[1 1 1] Functions for the black board
  (AI|Components|Blackboard|SetValueasObject (AI|GetBlackboard (AI|GetAIController self)) (Utilities|Name|MakeLiteralName "TargetActor") Actor))

(event Custom|Clear%20AI%20Target
  ;[1 1 1] Functions for the black board
  (AI|Components|Blackboard|ClearValue (AI|GetBlackboard (AI|GetAIController self)) (Utilities|Name|MakeLiteralName "TargetActor")))

(event Custom|Clear%20Camera%20Alarm
  ;[1 1 1] Functions for the camera alert
  (AI|Components|Blackboard|SetValueasBool (Variables|/Script/AIModule.AIController|GetBlackboard (AI|GetAIController self)) (Utilities|Name|MakeLiteralName "CameraAlarm") false)
  (Variables|/Script/Engine.CharacterMovementComponent|SetMaxWalkSpeed (Variables|Character|GetCharacterMovement) (Variables|Default|GetWalkingSpeed)))

(event Custom|Check%20If%20Is%20Office%20AI
  (if (Variables|Default|GetIsOfficeAI)
    (AI|Components|Blackboard|SetValueasBool (Variables|/Script/AIModule.AIController|GetBlackboard (AI|GetAIController self)) (Utilities|Name|MakeLiteralName "IsOfficeAI") true)))

(event EventBeginPlay
  (CallFunction|CheckifIsOfficeAI))

(fn ConstructionScript)

(fn HandleSight
  (params (Actor :type Actor%20Object%20Reference) (Stimulus :type AI%20Stimulus%20Structure))
  (bind _returnvalue (Class|AIPerceptionSystem|GetSenseClassforStimulus Stimulus))
  (if (== _returnvalue "/Script/AIModule.AISense_Sight")
    (if (== Actor (Game|GetPlayerCharacter 0))
      (AI|Components|Blackboard|SetValueasObject (AI|GetBlackboard (AI|GetAIController self)) (Utilities|Name|MakeLiteralName "TargetActor") (Utilities|SelectObject (Game|GetPlayerCharacter 0) 0 (.bsuccessfullysensed Stimulus)))
      (if (not (.bsuccessfullysensed Stimulus))
        (AI|Components|Blackboard|SetValueasVector (AI|GetBlackboard (AI|GetAIController self)) (Utilities|Name|MakeLiteralName "LastKnownLocation") (.stimuluslocation Stimulus)))
      (else
        (return)))
    (else
      (return))))